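; BP_Outline is an actor that shows a configurable static mesh and can toggle a colored outline around it.
; BeginPlay assigns the mesh, and CreateOutline spawns an unattached, slightly enlarged copy at its transform with a dynamic outline material fed color and scale.
; DeleteOutline destroys that copy, with a flag preventing duplicates.
; A player-distance check exists but is disconnected, so both events rely on external callers.
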(event Custom|CreateOutline
  (bind _mesh (Variables|Default|GetMesh))
  (bind _returnvalue (Transformation|GetWorldTransform _mesh))
  (if (not (Variables|Default|GetHasOutline))
    (bind _returnvalue_2 (AddComponent|AddStaticMeshComponent true (Math|Transform|MakeTransform (.location _returnvalue) (.rotation _returnvalue) "1.200000,1.200000,1.200000")))
    (bind _output_get (Variables|Default|SetOutlineMesh _returnvalue_2))
    (Components|StaticMesh|SetStaticMesh _output_get (Variables|Default|GetMeshVariable))
    (bind _returnvalue_3 (Rendering|Material|CreateDynamicMaterialInstance _output_get 0 "/Game/Materials/M_Outline_Inst.M_Outline_Inst" "" :!class /Script/Engine.PrimitiveComponent))
    (Rendering|Material|SetVectorParameterValue _returnvalue_3 "Color" (Variables|Default|GetOutlineColor) :!class /Script/Engine.MaterialInstanceDynamic)
    (Rendering|Material|SetScalarParameterValue _returnvalue_3 "Scale" (Variables|Default|GetScale) :!class /Script/Engine.MaterialInstanceDynamic)
    (Variables|Default|SetHasOutline true)))

(event Custom|DeleteOutline
  (bind _outlinemesh (Variables|Default|GetOutlineMesh))
  (Utilities|IsValid _outlinemesh
    (:Is%20Valid
      (Components|DestroyComponent _outlinemesh)
      (Variables|Default|SetHasOutline false))))

(event EventBeginPlay
  (Components|StaticMesh|SetStaticMesh (Variables|Default|GetMesh) (Variables|Default|GetMeshVariable)))

(event EventTick
  (params (DeltaSeconds :type Float%20%28single-precision%29))
  ;[0.007975 0.1094 0.01715] BWERF
)

(fn ConstructionScript)