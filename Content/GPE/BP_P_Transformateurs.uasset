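; Interactable transformer station that processes a resource passed to it by cooking it, cutting it or, in Vide mode, filling a bucket with its contents.
; Interact snaps the resource to an attach point, waits, applies the transformation, then launches it forward with sound and sparks.
; A timeline pulses the cube's scale at start and finish.
; Highlighting spawns a BP_Outline child actor from the cube's mesh, deleted on unhighlight.
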(event EventHightlight
  (Development|PrintString "Hello")
  (bind _returnvalue (AddComponent|AddChildActorComponent true (Transformation|GetWorldTransform (Variables|Default|GetCube))))
  (bind _asbp_outline (Utilities|Casting|CastToBP_Outline (Variables|/Script/Engine.ChildActorComponent|GetChildActor _returnvalue)))
  (Transformation|AttachActorToActor _asbp_outline 0 "None" "SnapToTarget" "SnapToTarget" "KeepRelative" true)
  (Variables|/Game/Materials/BP_Outline.BP_Outline_C|SetMeshVariable _asbp_outline (Variables|/Script/Engine.StaticMeshComponent|GetStaticMesh (Variables|Default|GetCube)))
  (Default|CreateOutline _asbp_outline))

(event EventStopHightlight
  (Default|DeleteOutline (stale EventHightlight _asbp_outline)))

(event EventInteract
  (params (Object :type BP%20P%20Takable%20Object%20Reference) (Player :type CH%20Player%20Object%20Reference))
  (bind _cube (Variables|Default|GetCube))
  (Utilities|FlowControl|Sequence
    (:then_0
      (bind _output_get (Variables|Default|SetRessourceToChange Object))
      (Physics|SetSimulatePhysics (Variables|/Game/Ressources/BP_P_Takable.BP_P_Takable_C|GetVisibleMesh _output_get) false)
      (Transformation|AttachComponentToComponent _output_get (Variables|Default|GetAttachLocation) "None" "SnapToTarget" "KeepRelative" "KeepRelative" true)
      (Audio|PlaySoundatLocation (Variables|Default|GetSoundProcess) (Transformation|GetWorldLocation (Variables|Default|GetCube)) "0, 0, 0" 1.0 1.0 0.0 0 0 0)
      (Utilities|FlowControl|Delay (Variables|Default|GetTimeToTransform))
      (Utilities|FlowControl|Sequence
        (:then_0
          (bind _asbp_p_ressources (Utilities|Casting|CastToBP_P_Ressources Object))
          (switch Utilities|FlowControl|Switch|SwitchonEnum_RessourceState (Variables|Default|GetTransformation)
            (:NewEnumerator1
              (Default|Cook _asbp_p_ressources))
            (:NewEnumerator2
              (Default|Cut _asbp_p_ressources))
            (:NewEnumerator4
              (Utilities|Casting|CastToBP_Seau _asbp_p_ressources
                (:then
                  (Default|Remplissage _asbp_p_ressources (Variables|Default|GetContenu)))
                (:CastFailed
                  _))))
          (CallFunction|Detachfrom)
          (Audio|PlaySoundatLocation "/Game/SoundMusics/Bruitages/Trasnfo_fini.Trasnfo_fini" (Transformation|GetWorldLocation _cube) "0, 0, 0" 1.0 1.0 0.0 0 0 0)
          (Niagara|SpawnSystematLocation "/Game/Vfxs/Systemes/NA_Sparks.NA_Sparks" (Transformation|GetWorldLocation _cube)))
        (:then_1
          (bind _scalevalue (Timeline|Timeline_0 PlayFromStart)
            (:Update
              (Transformation|SetWorldScale3D (Variables|Default|GetCube) (Math|Conversions|ToVector(Float) _scalevalue)))))))
    (:then_1
      (Timeline|Timeline_0 PlayFromStart))))

(fn ConstructionScript)

(fn Detachfrom
  (bind _ressourcetochange (Variables|Default|GetRessourceToChange))
  (bind _visiblemesh (Variables|/Game/Ressources/BP_P_Takable.BP_P_Takable_C|GetVisibleMesh _ressourcetochange))
  (Transformation|DetachFromActor _ressourcetochange "KeepWorld" "KeepWorld" "KeepRelative")
  (Physics|SetSimulatePhysics _visiblemesh true)
  (Physics|AddForce _visiblemesh (* (Math|Vector|GetForwardVector (Variables|Default|GetAttachLocation)) (* (Variables|Default|GetForceLancement) 1e+05)) "None" false)
  (Niagara|SpawnSystematLocation "/Game/Vfxs/Systemes/NA_Sparks.NA_Sparks" (Transformation|GetWorldLocation (Variables|Default|GetAttachLocation))))