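; Altar that accepts an interacting BP_Bol, snaps it in place, judges its food, then detaches it, marks it eaten and throws it forward.
; CheckIngredients appends the contents to FoodList, which is never cleared here, rejects empty or over-five lists and exact-matches two DT_Recettes rows.
; CheckAppreciation dispatches the rating to reaction functions that print and throw, with a sound for positive ratings.
; It reruns after any match, so reactions repeat.
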(event EventInteract
  (params (Object :type BP%20P%20Takable%20Object%20Reference) (Player :type CH%20Player%20Object%20Reference))
  (bind _asbp_bol (Utilities|Casting|CastToBP_Bol Object))
  (Variables|Default|SetBol _asbp_bol)
  (Physics|SetSimulatePhysics (Variables|/Game/Ressources/BP_P_Takable.BP_P_Takable_C|GetMesh _asbp_bol) false)
  (Transformation|AttachComponentToComponent Object (Variables|Default|GetLocation) "None" "SnapToTarget" "SnapToTarget" "KeepRelative" true)
  (Utilities|FlowControl|Delay 1.0)
  (CallFunction|CheckIngredients)
  ;[1 1 1] Finish To eat
  (Transformation|DetachFromActor Object "KeepWorld" "KeepWorld" "KeepRelative")
  (Default|BolEaten _asbp_bol)
  (CallFunction|Throw 5.0))

(fn ConstructionScript)

(fn CheckIngredients
  (Variables|Default|SetCurrentAppreciation "NewEnumerator4")
  (Utilities|Array|AppendArray (LocalVariables|GetFoodList) (Variables|/Game/GPE/BP_Bol.BP_Bol_C|GetRessourcesIn (Variables|Default|GetBol)))
  (if (<= (Utilities|Array|Length (LocalVariables|GetFoodList)) 0)
    (CallFunction|NotGood :!label _label)
    (elif (> (Utilities|Array|Length (LocalVariables|GetFoodList)) 5)
      (goto _label)
      (else
        (Utilities|FlowControl|Sequence
          (:then_0
            (bind _returnvalue (Utilities|GetDataTableRow "/Game/Ressources/DT_Recettes.DT_Recettes" "Oeuf")
              (:then
                (if (Utilities|Array|Identical (.Ingredients (Utilities|Struct|BreakStr_Recette _returnvalue)) (LocalVariables|GetFoodList))
                  (Development|PrintString "Oeuf pris")
                  (Variables|Default|SetCurrentAppreciation (.Appeciation (Utilities|Struct|BreakStr_Recette _returnvalue)))
                  (CallFunction|CheckAppreciation :!label _label_2)))))
          (:then_1
            (bind _returnvalue_2 (Utilities|GetDataTableRow "/Game/Ressources/DT_Recettes.DT_Recettes" "Patata")
              (:then
                (if (Utilities|Array|Identical (.Ingredients (Utilities|Struct|BreakStr_Recette _returnvalue_2)) (LocalVariables|GetFoodList))
                  (Development|PrintString "Oeuf+ Patates")
                  (Variables|Default|SetCurrentAppreciation (.Appeciation (Utilities|Struct|BreakStr_Recette _returnvalue_2)))
                  (goto _label_2)))))
          (:then_2
            (CallFunction|CheckAppreciation)))))))

(fn NotGood
  (Development|PrintString "Autel pas content")
  (CallFunction|Throw 2e+01))

(fn Good
  (Development|PrintString "Autel Good")
  (CallFunction|Throw 5.0))

(fn VeryGood
  (Development|PrintString "Autel Very Good")
  (CallFunction|Throw 5.0))

(fn Perfect
  (Development|PrintString "Autel Content")
  (CallFunction|Throw 5.0))

(fn Throw
  (params (Force :type Float%20%28single-precision%29))
  (bind _bol (Variables|Default|GetBol))
  (bind _mesh (Variables|/Game/Ressources/BP_P_Takable.BP_P_Takable_C|GetMesh _bol))
  (Physics|SetSimulatePhysics _mesh true)
  (Physics|AddForce _mesh (* (Math|Vector|GetForwardVector (Variables|Default|GetLocation)) (* Force 1e+05)) "None" false))

(fn CheckAppreciation
  (switch Utilities|FlowControl|Switch|SwitchonEnum_Appreciation (Variables|Default|GetCurrentAppreciation)
    (:NewEnumerator4
      (Development|PrintString "Neutre"))
    (:NewEnumerator0
      (CallFunction|NotGood))
    (:NewEnumerator1
      (CallFunction|Good)
      (Audio|PlaySoundatLocation "/Game/SoundMusics/Bruitages/Rot.Rot" (Transformation|GetWorldLocation (Variables|Default|GetCube)) "0, 0, 0" 1.0 1.0 0.0 0 0 0 :!label _label))
    (:NewEnumerator2
      (CallFunction|VeryGood)
      (goto _label))
    (:NewEnumerator3
      (CallFunction|Perfect)
      (goto _label))))