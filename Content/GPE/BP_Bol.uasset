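; BP_Bol is a bowl that collects food resources through interaction and holds them until it is eaten.
; Interacting with a BP_P_Ressources object records its food type and state in RessourcesIn.
; A bucket (BP_Seau) is emptied via Vider and kept, while any other resource actor is destroyed.
; The BolEaten event clears the stored contents.
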(event Custom|BolEaten
  (Utilities|Array|Clear (Variables|Default|GetRessourcesIn)))

(event EventInteract
  (params (Object :type BP%20P%20Takable%20Object%20Reference))
  (Utilities|IsValid Object
    (:Is%20Valid
      (bind _asbp_p_ressources (Utilities|Casting|CastToBP_P_Ressources Object))
      (Utilities|Array|Add (Variables|Default|GetRessourcesIn) (Utilities|Struct|MakeStr_FoodInfo (Variables|/Game/Ressources/BP_P_Ressources.BP_P_Ressources_C|GetFoodType _asbp_p_ressources) (Variables|/Game/Ressources/BP_P_Ressources.BP_P_Ressources_C|GetState _asbp_p_ressources)))
      (bind _asbp_seau (Utilities|Casting|CastToBP_Seau Object)
        (:then
          (Default|Vider _asbp_seau))
        (:CastFailed
          (Actor|DestroyActor Object))))))

(fn ConstructionScript)