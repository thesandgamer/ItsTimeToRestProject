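; Interactable fishing rod that produces a fish and flings it out of the water.
; On Interact it plays a rod sound, waits a delay, then spawns BP_Poisson at its Arrow and launches it with a physics force scaled by ForceLancer, adding a splash effect and sound.
; Highlight events create and delete a BP_Outline child actor copying the rod's static mesh.
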(event EventInteract
  (params (Object :type BP%20P%20Takable%20Object%20Reference) (Player :type CH%20Player%20Object%20Reference))
  (bind _arrow (Variables|Default|GetArrow))
  (Audio|PlaySoundatLocation "/Game/SoundMusics/Bruitages/Fishing_rod.Fishing_rod" (Transformation|GetWorldLocation (Variables|Default|GetStaticMesh)) "0, 0, 0" 1.0 1.0 0.0 0 0 0)
  ;[1 1 1] On recoit le message, on attend quelques segondes(un peut de random, et un poisson spawn au bout de la ligne et est balancé vers le pole
  (Utilities|FlowControl|Delay (Variables|Default|GetDuration))
  (bind _returnvalue (Game|SpawnActorfromClass "/Game/Ressources/Nourritures/BP_Poisson.BP_Poisson_C" (Math|Transform|MakeTransform (Transformation|GetWorldLocation _arrow) "0, 0, 0" "1,1,1") "Undefined" 0 "NewEnumerator6" self 0))
  (Physics|SetSimulatePhysics (Variables|/Game/Ressources/BP_P_Takable.BP_P_Takable_C|GetVisibleMesh _returnvalue) true)
  (Physics|AddForce (Variables|/Game/Ressources/BP_P_Takable.BP_P_Takable_C|GetVisibleMesh _returnvalue) (* (Math|Vector|GetForwardVector _arrow) (* 1e+06 (Variables|Default|GetForceLancer))) "None" false)
  (Audio|PlaySoundatLocation "/Game/SoundMusics/Bruitages/Fish_out.Fish_out" (Transformation|GetWorldLocation (Variables|Default|GetStaticMesh)) "0, 0, 0" 1.0 1.0 0.0 0 0 0)
  (Niagara|SpawnSystematLocation "/Game/Vfxs/Systemes/NA_WaterSplash.NA_WaterSplash" (Transformation|GetWorldLocation (Variables|Default|GetArrow))))

(event EventHightlight
  (Development|PrintString "Hello")
  (bind _returnvalue (AddComponent|AddChildActorComponent true (Transformation|GetWorldTransform (Variables|Default|GetStaticMesh))))
  (bind _asbp_outline (Utilities|Casting|CastToBP_Outline (Variables|/Script/Engine.ChildActorComponent|GetChildActor _returnvalue)))
  (Transformation|AttachActorToActor _asbp_outline 0 "None" "SnapToTarget" "SnapToTarget" "KeepRelative" true)
  (Variables|/Game/Materials/BP_Outline.BP_Outline_C|SetMeshVariable _asbp_outline (Variables|/Script/Engine.StaticMeshComponent|GetStaticMesh (Variables|Default|GetStaticMesh)))
  (Default|CreateOutline _asbp_outline))

(event EventStopHightlight
  (Default|DeleteOutline (stale EventHightlight _asbp_outline)))

(fn ConstructionScript)