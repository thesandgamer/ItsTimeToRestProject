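; Resource actor with a preparation state (raw, cooked, cut, cooked-and-cut, water) that frees its linked spawner when interacted with.
; Cook and Cut advance the state enum, converging on cooked-and-cut in either order, print it, then call ChangeMeshs to swap the static mesh from a four-entry array.
; Remplissage (filling) turns a raw resource to water without updating the mesh.
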(event EventInteract
  (params (Object :type BP%20P%20Takable%20Object%20Reference))
  (bind _spawnerlinkto (Variables|Default|GetSpawnerLinkTo))
  (Utilities|IsValid _spawnerlinkto
    (:Is%20Valid
      (Variables|/Game/Ressources/Bp_P_Spawner.Bp_P_Spawner_C|SetHasSpawn _spawnerlinkto false))))

(fn ConstructionScript)

(fn Cook
  (switch Utilities|FlowControl|Switch|SwitchonEnum_RessourceState (Variables|Default|GetState)
    (:NewEnumerator0
      (Variables|Default|SetState "NewEnumerator1")
      (Development|PrintString "Cuit"))
    (:NewEnumerator2
      (Variables|Default|SetState "NewEnumerator3")
      (Development|PrintString "CuitCoupé")))
  (CallFunction|ChangeMeshs))

(fn Cut
  (switch Utilities|FlowControl|Switch|SwitchonEnum_RessourceState (Variables|Default|GetState)
    (:NewEnumerator0
      (Variables|Default|SetState "NewEnumerator2")
      (Development|PrintString "Coupé"))
    (:NewEnumerator1
      (Variables|Default|SetState "NewEnumerator3")
      (Development|PrintString "CoupéCuit")))
  (CallFunction|ChangeMeshs))

(fn ChangeMeshs
  (bind _mesh (Variables|Character|GetMesh))
  (bind _meshs (Variables|Default|GetMeshs))
  (if (> (Utilities|Array|Length (Variables|Default|GetMeshs)) 3)
    (switch Utilities|FlowControl|Switch|SwitchonEnum_RessourceState (Variables|Default|GetState)
      (:NewEnumerator0
        (Components|StaticMesh|SetStaticMesh _mesh (Utilities|Array|Get(acopy) _meshs)))
      (:NewEnumerator1
        (Components|StaticMesh|SetStaticMesh _mesh (Utilities|Array|Get(acopy) _meshs 1)))
      (:NewEnumerator2
        (Components|StaticMesh|SetStaticMesh _mesh (Utilities|Array|Get(acopy) _meshs 2)))
      (:NewEnumerator3
        (Components|StaticMesh|SetStaticMesh _mesh (Utilities|Array|Get(acopy) _meshs 3))))))

(fn Remplissage
  (switch Utilities|FlowControl|Switch|SwitchonEnum_RessourceState (Variables|Default|GetState)
    (:NewEnumerator0
      (Variables|Default|SetState "NewEnumerator4"))))