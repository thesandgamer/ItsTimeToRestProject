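; Spawner actor that places a resource pickup, such as food, at its spawn point.
; A looping timer started on BeginPlay spawns the configured class at the SpawnLocation component whenever nothing has been spawned yet.
; The spawned BP_P_Ressources receives a link back to this spawner, and a HasSpawn flag blocks further spawns while it stays set.
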(event Custom|Spawn
  (if (not (Variables|Default|GetHasSpawn))
    (bind _returnvalue (Game|SpawnActorfromClass (Variables|Default|GetFoodToSpawn) (Transformation|GetWorldTransform (Variables|Default|GetSpawnLocation)) "Undefined" 0 0))
    (bind _asbp_p_ressources (Utilities|Casting|CastToBP_P_Ressources _returnvalue))
    (Variables|/Game/Ressources/BP_P_Ressources.BP_P_Ressources_C|SetSpawnerLinkTo _asbp_p_ressources self)
    (Variables|Default|SetHasSpawn true)))

(event EventBeginPlay
  (Utilities|Time|SetTimerbyEvent (delegate Custom|Spawn) 7.0 true))

(fn ConstructionScript)