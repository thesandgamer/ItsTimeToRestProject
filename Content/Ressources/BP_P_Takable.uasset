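; BP_P_Takable is a physics-simulated prop, named as takable, that can be highlighted with an outline.
; On BeginPlay it enables physics on VisibleMesh.
; Hightlight prints a debug string, spawns a child actor component, attaches its BP_Outline to itself, passes it the static mesh and calls CreateOutline.
; StopHightlight is empty; the DeleteOutline call is unconnected, so outlines are never removed here.
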(event EventBeginPlay
  (Physics|SetSimulatePhysics (Variables|Default|GetVisibleMesh) true))

(event EventHightlight
  (Development|PrintString "Hello")
  (bind _returnvalue (AddComponent|AddChildActorComponent true (Transformation|GetWorldTransform (Variables|Default|GetVisibleMesh))))
  (bind _asbp_outline (Utilities|Casting|CastToBP_Outline (Variables|/Script/Engine.ChildActorComponent|GetChildActor _returnvalue)))
  (Transformation|AttachActorToActor _asbp_outline self "None" "SnapToTarget" "SnapToTarget" "KeepRelative" true)
  (Variables|/Game/Materials/BP_Outline.BP_Outline_C|SetMeshVariable _asbp_outline (Variables|/Script/Engine.StaticMeshComponent|GetStaticMesh (Variables|Default|GetVisibleMesh)))
  (Default|CreateOutline _asbp_outline))

(event EventStopHightlight)

(fn ConstructionScript)